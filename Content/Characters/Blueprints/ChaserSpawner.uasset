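; Spawner actor that periodically creates Chaser AI pawns at its own location.
; A looping timer started on BeginPlay fires SpawnChaser every few seconds, which spawns only while the ChasersAreSpawning flag is set.
; A separate Turn180 function, not called within this Blueprint, flips the actor's rotation by special-casing zero and half-turn values and negating any other rotation.
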(event Custom|SpawnChaser
  (if (Variables|Default|GetChasersAreSpawning)
    (AI|SpawnAIFromClass "/Game/Characters/Blueprints/Chaser.Chaser_C" 0 (Transformation|GetActorLocation) "0, 0, 0" false 0)))

(event EventBeginPlay
  (Utilities|Time|SetTimerbyEvent (delegate Custom|SpawnChaser) 3.0 true))

(event Collision|EventActorBeginOverlap
  (params (OtherActor :type Actor%20Object%20Reference)))

(fn ConstructionScript)

(fn Turn180
  (bind _returnvalue (Transformation|GetActorRotation))
  (if (Utilities|Operators|EqualEqual :B _returnvalue)
    (Transformation|SetActorRotation "0.000000,180.000000,0.000000")
    (elif (Utilities|Operators|EqualEqual "0.000000,180.000000,0.000000" _returnvalue 0.0)
      (Transformation|SetActorRotation "0.000000,360.000000,0.000000")
      (else
        (Transformation|SetActorRotation (* _returnvalue -1.0))))))