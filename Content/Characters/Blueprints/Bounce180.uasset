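; Bounce180 is a sprite-based patrolling hazard character that walks back and forth and damages the player on overlap.
; A looping timer started at BeginPlay repeatedly adds movement input along the sprite's forward vector.
; Any hit calls Turn180, which reverses facing by comparing and setting exact actor rotations.
; Overlaps with actors tagged as the player apply damage to player character zero and print the result.
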(event Custom|MoveForward
  (Pawn|Input|AddMovementInput (Math|Vector|GetForwardVector (Variables|Default|GetSprite)) 1.0 false))

(event EventBeginPlay
  (Utilities|Time|SetTimerbyEvent (delegate Custom|MoveForward) 0.03 true))

(event Collision|EventActorBeginOverlap
  (params (OtherActor :type Actor%20Object%20Reference))
  (if (Actor|ActorHasTag OtherActor "PlayerCharacterTag")
    (bind _returnvalue (Game|Damage|ApplyDamage (Game|GetPlayerCharacter 0) 1.0 0 0 "/Script/Engine.DamageType"))
    (Development|PrintString (Utilities|String|ToString(Float) _returnvalue))))

(event EventTick
  (params (DeltaSeconds :type Float%20%28single-precision%29)))

(event Collision|EventHit
  (params (MyComp :type Primitive%20Component%20Object%20Reference) (Other :type Actor%20Object%20Reference) (OtherComp :type Primitive%20Component%20Object%20Reference) (bSelfMoved :type Boolean) (HitLocation :type Vector :default "0, 0, 0") (HitNormal :type Vector :default "0, 0, 0") (NormalImpulse :type Vector :default "0, 0, 0") (Hit :type Hit%20Result%20Structure%20%28by%20ref%29))
  (CallFunction|Turn180))

(fn ConstructionScript)

(fn Turn180
  (bind _returnvalue (Transformation|GetActorRotation))
  (if (Utilities|Operators|EqualEqual :B _returnvalue)
    (Transformation|SetActorRotation "0.000000,180.000000,0.000000")
    (elif (Utilities|Operators|EqualEqual "0.000000,180.000000,0.000000" _returnvalue 0.0)
      (Transformation|SetActorRotation "0.000000,360.000000,0.000000")
      (else
        (Transformation|SetActorRotation (* _returnvalue -1.0))))))