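; Collectible chip actor that the player character picks up by touching it.
; On overlap, it casts the other actor's instigator to CharBlueprint, increments that character's ChipCounter, prints the count and destroys itself.
; A separate Turn 180 function, not called within this Blueprint, flips the chip between zero and half-turn rotations by exact comparison, negating any other rotation.
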(event Collision|EventActorBeginOverlap
  (params (OtherActor :type Actor%20Object%20Reference))
  (bind _aschar_blueprint (Utilities|Casting|CastToCharBlueprint (Game|GetInstigator OtherActor)))
  (bind _result (Math|Integer|IncrementInt (Variables|/Game/Characters/Blueprints/CharBlueprint.CharBlueprint_C|GetChipCounter _aschar_blueprint))
    (:%20%20
      (Development|PrintString (Utilities|String|ToString(Integer) _result))
      (Actor|DestroyActor))))

(fn ConstructionScript)

(fn Turn180
  (bind _returnvalue (Transformation|GetActorRotation))
  (if (Utilities|Operators|EqualEqual :B _returnvalue)
    (Transformation|SetActorRotation "0.000000,180.000000,0.000000")
    (elif (Utilities|Operators|EqualEqual "0.000000,180.000000,0.000000" _returnvalue 0.0)
      (Transformation|SetActorRotation "0.000000,360.000000,0.000000")
      (else
        (Transformation|SetActorRotation (* _returnvalue -1.0))))))