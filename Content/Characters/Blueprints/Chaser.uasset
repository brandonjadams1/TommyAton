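; Sprite-based enemy character that chases the player and deals damage on contact.
; A looping timer periodically turns it to face player 0 and adds one pulse of movement input along the sprite's forward vector.
; Overlapping an actor tagged as the player applies damage to player 0 and prints the result.
; A Turn180 helper flips the actor's rotation but is not called in this graph.
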(event Custom|MoveForward
  (Transformation|SetActorRotation (Math|Rotator|FindLookatRotation (Transformation|GetActorLocation) (Transformation|GetActorLocation (Game|GetPlayerCharacter 0))))
  (Pawn|Input|AddMovementInput (Math|Vector|GetForwardVector (Variables|Default|GetSprite)) 1.0 false))

(event EventBeginPlay
  (Utilities|Time|SetTimerbyEvent (delegate Custom|MoveForward) 0.3 true))

(event Collision|EventActorBeginOverlap
  (params (OtherActor :type Actor%20Object%20Reference))
  (if (Actor|ActorHasTag OtherActor "PlayerCharacterTag")
    (bind _returnvalue (Game|Damage|ApplyDamage (Game|GetPlayerCharacter 0) 1.0 0 0 "/Script/Engine.DamageType"))
    (Development|PrintString (Utilities|String|ToString(Float) _returnvalue))))

(fn ConstructionScript)

(fn Turn180
  (bind _returnvalue (Transformation|GetActorRotation))
  (if (Utilities|Operators|EqualEqual :B _returnvalue)
    (Transformation|SetActorRotation "0.000000,180.000000,0.000000")
    (elif (Utilities|Operators|EqualEqual "0.000000,180.000000,0.000000" _returnvalue 0.0)
      (Transformation|SetActorRotation "0.000000,360.000000,0.000000")
      (else
        (Transformation|SetActorRotation (* _returnvalue -1.0))))))