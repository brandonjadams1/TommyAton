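; Player character Blueprint with a flipbook sprite that moves, jumps and ends the game on taking any damage.
; BeginPlay adds the Enhanced Input mapping context, whose actions drive movement along the control rotation's forward vector and jumping.
; Each Tick picks the jump, fall, run or idle flipbook from velocity and falling state.
; Damage pauses the game and replaces all widgets with a Game Over screen.
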(event Input|EnhancedActionEvents|EnhancedInputActionIA_Move
  (params (ActionValue :type Float%20%28double-precision%29) (ElapsedSeconds :type Float%20%28double-precision%29) (TriggeredSeconds :type Float%20%28double-precision%29) (InputAction :type Input%20Action%20Object%20Reference :default "/Game/UI/IA_Move.IA_Move"))
  (:Triggered
    (Pawn|Input|AddMovementInput (Math|Vector|GetForwardVector (Pawn|GetControlRotation :!class /Script/Engine.Pawn)) ActionValue false))
  (:Completed
    (Variables|Default|SetbUseControllerRotationYaw false)))

(event Input|EnhancedActionEvents|EnhancedInputActionIA_Jump
  (params (ActionValue :type Boolean) (ElapsedSeconds :type Float%20%28double-precision%29) (TriggeredSeconds :type Float%20%28double-precision%29) (InputAction :type Input%20Action%20Object%20Reference :default "/Game/UI/IA_Jump.IA_Jump"))
  (:Triggered
    (Character|Jump)))

(event EventBeginPlay
  (|SetUpMappingContext))

(event Game|Damage|EventAnyDamage
  (params (Damage :type Float%20%28single-precision%29) (DamageType :type Damage%20Type%20Object%20Reference) (InstigatedBy :type Controller%20Object%20Reference) (DamageCauser :type Actor%20Object%20Reference))
  (CallFunction|GameOver))

(event EventTick
  (params (DeltaSeconds :type Float%20%28single-precision%29))
  (|SetAnimations))

(fn ConstructionScript)

(fn GameOver
  (Game|SetGamePaused true)
  (Viewport|RemoveAllWidgets)
  (bind _returnvalue (UserInterface|CreateWidget "/Game/UI/GameOverScreen.GameOverScreen_C" (Game|GetPlayerController 0)))
  (UserInterface|Viewport|AddtoViewport _returnvalue 0))