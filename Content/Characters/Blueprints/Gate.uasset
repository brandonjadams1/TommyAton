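; Level exit gate that clears the level when a player character carrying enough chips overlaps it.
; On overlap it casts the other actor's instigator to CharBlueprint and compares its ChipCounter with ChipsNeeded, set on BeginPlay.
; LevelCleared pauses the game and replaces all widgets with the level-cleared screen.
; It also defines a similar GameOver screen function and a Turn180 rotation helper, neither called within this Blueprint.
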(event EventBeginPlay
  (Variables|Default|SetChipsNeeded 3))

(event Collision|EventActorBeginOverlap
  (params (OtherActor :type Actor%20Object%20Reference))
  (bind _aschar_blueprint (Utilities|Casting|CastToCharBlueprint (Game|GetInstigator OtherActor)))
  (if (>= (Variables|/Game/Characters/Blueprints/CharBlueprint.CharBlueprint_C|GetChipCounter _aschar_blueprint) (Variables|Default|GetChipsNeeded))
    (|LevelCleared)))

(fn ConstructionScript)

(fn Turn180
  (bind _returnvalue (Transformation|GetActorRotation))
  (if (Utilities|Operators|EqualEqual :B _returnvalue)
    (Transformation|SetActorRotation "0.000000,180.000000,0.000000")
    (elif (Utilities|Operators|EqualEqual "0.000000,180.000000,0.000000" _returnvalue 0.0)
      (Transformation|SetActorRotation "0.000000,360.000000,0.000000")
      (else
        (Transformation|SetActorRotation (* _returnvalue -1.0))))))

(fn GameOver
  (Game|SetGamePaused true)
  (Viewport|RemoveAllWidgets)
  (bind _returnvalue (UserInterface|CreateWidget "/Game/UI/GameOverScreen.GameOverScreen_C" (Game|GetPlayerController 0)))
  (UserInterface|Viewport|AddtoViewport _returnvalue 0))